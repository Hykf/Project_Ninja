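; BP_Kunai is a kunai projectile that deals physical damage on contact and destroys itself.
; When its collision begins overlapping, a short forward line trace for one object type decides whether the player's DealDamage is applied to the overlapped actor.
; A failed trace instead halts the projectile and spawns a fire vanquish Niagara effect before destruction.
; End overlap restores collision, gravity and movement.
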(event `self.ReceiveBeginPlay`)

(event `self.ReceiveTick`
  (params (DeltaSeconds :type "Float (single-precision)")))

(event `self.KunaiCollision.OnComponentBeginOverlap`
  (params (OverlappedComponent :type "PrimitiveComponent Object Reference") (OtherActor :type "Actor Object Reference") (OtherComp :type "PrimitiveComponent Object Reference") (OtherBodyIndex :type Integer) (bFromSweep :type Boolean) (SweepResult :type "HitResult Structure (by ref)"))
  (bind _returnvalue (`self.K2_GetActorLocation`))
  (bind (_outhit _returnvalue_2) (`KismetSystemLibrary.LineTraceSingleForObjects` _returnvalue (+ _returnvalue (* (`self.GetActorForwardVector`) 100.0)) (`|MakeArray` "ObjectTypeQuery7" :!type "EObjectTypeQuery Enum")))
  (if _returnvalue_2
    (`/Game/Blueprints/Characters/BP_MainCharacter.Deal Damage` (`self.Player`) OtherActor "Physical" 10.0)
    (`self.K2_DestroyActor`)
    (else
      (set `MovementComponent.Velocity` (0.0 0.0 0.0) (`self.ProjectileMovement`))
      (`PrimitiveComponent.SetEnableGravity` (`self.KunaiSprite`) false)
      (`ActorComponent.Deactivate` (`self.ProjectileMovement`))
      (`NiagaraFunctionLibrary.SpawnSystemAtLocation` "/Game/PixelArt/Character/Main/NS_FireVanquish.NS_FireVanquish" (`self.K2_GetActorLocation`))
      (`self.K2_DestroyActor`))))

(event `self.KunaiCollision.OnComponentEndOverlap`
  (params (OverlappedComponent :type "PrimitiveComponent Object Reference") (OtherActor :type "Actor Object Reference") (OtherComp :type "PrimitiveComponent Object Reference") (OtherBodyIndex :type Integer))
  (`PrimitiveComponent.SetCollisionEnabled` (`self.KunaiCollision`) "QueryAndPhysics")
  (`PrimitiveComponent.SetEnableGravity` (`self.KunaiSprite`) true)
  (`ActorComponent.Activate` (`self.ProjectileMovement`) false))

(fn `UserConstructionScript`
  (locals (NewLocalVar :type "/Game/Blueprints/Characters/BP_MainCharacter Object Reference")))