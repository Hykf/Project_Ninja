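; Village manager Blueprint that looks up merchant upgrade data by name.
; GetMerchantCurrentLevel searches the MerchantUpgrades array in VillUpgr and returns the matching entry's current level, or -1 when none matches.
; GetMerchantUpgradeCost runs the same search for upgrade cost, but its -1 fallback is unconnected and never runs.
; BeginPlay and the construction script are empty.
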(event `self.ReceiveBeginPlay`)

(fn `GetMerchantCurrentLevel`
  (params (Name :type String))
  (returns (CurrentLevel :type Integer))
  (for _array_element (`VillageUpgradeDataAsset.MerchantUpgrades` (`self.VillUpgr`))
    (bind ((`Name` _name) (`CurrentLevel` _currentlevel)) (break `MerchantUpgrade` _array_element))
    (if (== (`local.Name`) _name)
      (return _currentlevel)))
  (return -1))

(fn `GetMerchantUpgradeCost`
  (params (Name :type String))
  (returns (UpgradeCost :type Integer))
  (for _array_element (`VillageUpgradeDataAsset.MerchantUpgrades` (`self.VillUpgr`))
    (bind ((`Name` _name) (`UpgradeCost` _upgradecost)) (break `MerchantUpgrade` _array_element))
    (if (== (`local.Name`) _name)
      (return _upgradecost))))

(fn `UserConstructionScript`)