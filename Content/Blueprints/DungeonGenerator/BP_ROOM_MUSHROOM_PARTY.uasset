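; Mushroom party room for the dungeon generator, a tilemap room that stays dark until the player enters it.
; On BeginPlay it runs the parent logic, assigns its floor tilemap and tints floor and wall tilemaps black.
; Player overlap with the shadow collision marks it visited, restores white tint and fades the shadow's material through a timeline before destroying it.
; A delayed random loop after tilemap setup has an empty body.
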(event `self.ReceiveBeginPlay`
  ;[1 1 1] Podlacz jak naprawisz tilemapy
  (`parent.ReceiveBeginPlay`)
  (`|ExecutionSequence`
    (:`then_0`
      (`PaperTileMapComponent.SetTileMap` (`self.TileMapComponent`) (`KismetArrayLibrary.Array_Random` (`|MakeArray` "/Game/PixelArt/Background/RoomsAssets/TM_DungRoom5.TM_DungRoom5" :!type "PaperTileMap Object Reference")))
      (`KismetSystemLibrary.Delay` 0.2)
      (if (== (`KismetMathLibrary.RandomInteger` 1) 0)
        (for _ (range (+ (`KismetMathLibrary.RandomIntegerInRange` 1 3) 1))
          _)))
    (:`then_1`
      (`self.BeginColor`))))

(event `self.ShadowCollision_0.OnComponentBeginOverlap`
  (params (OverlappedComponent :type "PrimitiveComponent Object Reference") (OtherActor :type "Actor Object Reference") (OtherComp :type "PrimitiveComponent Object Reference") (OtherBodyIndex :type Integer) (bFromSweep :type Boolean) (SweepResult :type "HitResult Structure (by ref)"))
  (bind _roomshadow_0 (`self.RoomShadow_0`))
  (cast `/Game/Blueprints/Characters/BP_MainCharacter` OtherActor)
  (`/Engine/EditorBlueprintResources/StandardMacros.IsValid` _roomshadow_0
    (:`Is Valid`
      (bind _returnvalue (`PrimitiveComponent.CreateDynamicMaterialInstance` _roomshadow_0 0 (`PrimitiveComponent.GetMaterial` _roomshadow_0 0) "None"))
      (set `self.Visited_0` true)
      (`self.Visit`)
      (bind (_direction _powertrack) (`Timeline|Timeline_0`)
        (:`Update`
          (`MaterialInstanceDynamic.SetScalarParameterValue` _returnvalue "Power" _powertrack))
        (:`Finished`
          (`ActorComponent.K2_DestroyComponent` (`self.RoomShadow_0`)))))))

(event `Visit`
  (for _array_element (`|MakeArray` (`self.TileMapComponent`) (`self.TileMapComponentWallDown`) (`self.TileMapComponentWallRight`) (`self.TileMapComponentWallLeft`) (`self.TileMapComponentWallUp`))
    (`PaperTileMapComponent.SetTileMapColor` _array_element (struct :`R` 1.0 :`G` 1.0 :`B` 1.0 :`A` 1.0))))

(event `BeginColor`
  (for _array_element (`|MakeArray` (`self.TileMapComponent`) (`self.TileMapComponentWallDown`) (`self.TileMapComponentWallRight`) (`self.TileMapComponentWallLeft`) (`self.TileMapComponentWallUp`))
    (`PaperTileMapComponent.SetTileMapColor` _array_element (struct :`A` 1.0))))

(fn `UserConstructionScript`)