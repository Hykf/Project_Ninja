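; BP_RoomEnd is the dungeon generator's end room, which hosts the boss fight.
; When the main character first overlaps BossRoomInteract, the room shows its four wall tilemaps and removes that trigger.
; After a one-second delay it spawns a double-scale BP_Boss at the BPMoney component's location and adds a boss health bar widget bound to it.
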(event `self.ReceiveBeginPlay`)

(event `self.BossRoomInteract.OnComponentBeginOverlap`
  (params (OverlappedComponent :type "PrimitiveComponent Object Reference") (OtherActor :type "Actor Object Reference") (OtherComp :type "PrimitiveComponent Object Reference") (OtherBodyIndex :type Integer) (bFromSweep :type Boolean) (SweepResult :type "HitResult Structure (by ref)"))
  (cast `/Game/Blueprints/Characters/BP_MainCharacter` OtherActor)
  (`/Engine/EditorBlueprintResources/StandardMacros.DoOnce` false
    (:`Completed`
      (`self.BossInit`)
      (`ActorComponent.K2_DestroyComponent` (`self.BossRoomInteract`)))))

(event `BossInit`
  (for _array_element (`|MakeArray` (`self.TileMapComponentWallRight`) (`self.TileMapComponentWallDown`) (`self.TileMapComponentWallUp`) (`self.TileMapComponentWallLeft`))
    (`self.ChangeVisibility` _array_element true))
  (`KismetSystemLibrary.Delay` 1.0)
  (bind _returnvalue (`|SpawnActorFromClass` "/Game/Blueprints/AI/BP_Boss.BP_Boss_C" (`KismetMathLibrary.MakeTransform` (`SceneComponent.K2_GetComponentLocation` (`self.BP_Money`)) (struct) (2.0 2.0 2.0)) "AlwaysSpawn" "MultiplyWithRoot" null null))
  (bind _returnvalue_2 (`|CreateWidget` "/Game/Blueprints/Widgets/WBP_BossHealthBar.WBP_BossHealthBar_C" null _returnvalue))
  (`UserWidget.AddToViewport` _returnvalue_2 0))

(fn `UserConstructionScript`)