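; BP_Room is a dungeon generator room made of tilemaps that stays blacked out until the main character first enters.
; Entering restores tilemap color, fades the shadow through a material timeline, closes the wall doors and spawns enemies near random child spawn points on the XZ plane.
; A recursive delayed check prunes dead enemies and restores saved door visibility once the room is clear.
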(event `self.ReceiveBeginPlay`
  ;[1 1 1] Podlacz jak naprawisz tilemapy
  (`parent.ReceiveBeginPlay`)
  (`|ExecutionSequence`
    (:`then_1`
      (`self.BeginColor`))))

(event `self.ShadowCollision.OnComponentBeginOverlap`
  (params (OverlappedComponent :type "PrimitiveComponent Object Reference") (OtherActor :type "Actor Object Reference") (OtherComp :type "PrimitiveComponent Object Reference") (OtherBodyIndex :type Integer) (bFromSweep :type Boolean) (SweepResult :type "HitResult Structure (by ref)"))
  (bind _roomshadow (`self.RoomShadow`))
  (if (not (`self.Visited`))
    (cast `/Game/Blueprints/Characters/BP_MainCharacter` OtherActor)
    (`/Engine/EditorBlueprintResources/StandardMacros.IsValid` _roomshadow
      (:`Is Valid`
        (`self.SpawnEnemies`)
        (`self.CheckPresen`)
        (bind _returnvalue (`PrimitiveComponent.CreateDynamicMaterialInstance` _roomshadow 0 (`PrimitiveComponent.GetMaterial` _roomshadow 0) "None"))
        (`PrimitiveComponent.SetCollisionEnabled` (`self.ShadowCollision`) "NoCollision")
        (set `self.Visited` true)
        (`self.Visit`)
        (bind (_direction _powertrack) (`Timeline|Timeline`)
          (:`Update`
            (`MaterialInstanceDynamic.SetScalarParameterValue` _returnvalue "Power" _powertrack))
          (:`Finished`
            (`ActorComponent.K2_DestroyComponent` (`self.RoomShadow`))))))))

(event `Visit`
  ;[1 1 1] Color
  (for _array_element (`|MakeArray` (`self.TileMapComponent`) (`self.TileMapComponentWallDown`) (`self.TileMapComponentWallRight`) (`self.TileMapComponentWallLeft`) (`self.TileMapComponentWallUp`))
    (`PaperTileMapComponent.SetTileMapColor` _array_element (struct :`R` 1.0 :`G` 1.0 :`B` 1.0 :`A` 1.0))))

(event `CheckPresen`
  (`KismetSystemLibrary.Delay` 3.0)
  (for _array_element (`self.EnemiesInRoom`)
    (`KismetSystemLibrary.PrintString` (`KismetSystemLibrary.GetDisplayName` _array_element) true true (struct :`R` 1.0 :`B` 0.078669 :`A` 1.0))
    (if (not (`KismetSystemLibrary.IsValid` _array_element))
      (`KismetArrayLibrary.Array_RemoveItem` (`self.EnemiesInRoom`) _array_element)))
  (if (!= (`KismetArrayLibrary.Array_Length` (`self.EnemiesInRoom`)) 0)
    (`self.CheckPresen`)
    (else
      (`self.OpenCloseDoor` true))))

(event `BeginColor`
  ;[1 1 1] Color
  (for _array_element (`|MakeArray` (`self.TileMapComponent`) (`self.TileMapComponentWallDown`) (`self.TileMapComponentWallRight`) (`self.TileMapComponentWallLeft`) (`self.TileMapComponentWallUp`))
    (`PaperTileMapComponent.SetTileMapColor` _array_element (struct :`A` 1.0))))

(fn `OpenCloseDoor`
  (params (Open :type Boolean))
  (if Open
    (for (_array_element _array_index) (`self.Doors`)
      (`self.ChangeVisibility` _array_element (`|GetArrayItem` (`self.BeforeClosed`) _array_index)))
    (else
      (set `self.BeforeClosed` (`|MakeArray` (`self.RoofVisibility`) (`self.FloorVisibility`) (`self.LeftWallVisibility`) (`self.RightWallVisibility`)))
      (for _array_element_2 (`self.Doors`)
        (`self.ChangeVisibility` _array_element_2 true)))))

(fn `SpawnEnemies`
  (locals (EnemyClass :type "EnemyBase Class Reference") (SpawnPoints :type "Array of /Game/Blueprints/DungeonGenerator/BP_SpawnPoint Object Reference"))
  (bind _value (`BlueprintMapLibrary.Map_Find` (`self.Enemies`) (`local.EnemyClass`)))
  (bind (_x _y _z) (`KismetMathLibrary.BreakVector3f` (`SceneComponent.K2_GetComponentLocation` (`Actor.RootComponent` (`KismetArrayLibrary.Array_Random` (`local.SpawnPoints`))))))
  (`|ExecutionSequence`
    (:`then_0`
      (for _array_element (`self.GetAllChildActors` self true)
        (bind _asbp_spawn_point (cast `/Game/Blueprints/DungeonGenerator/BP_SpawnPoint` _array_element))
        (`KismetArrayLibrary.Array_Add` (`local.SpawnPoints`) _asbp_spawn_point)))
    (:`then_1`
      (`self.OpenCloseDoor` false)
      (bind _keys (`BlueprintMapLibrary.Map_Keys` (`self.Enemies`)))
      (for _array_element_2 _keys
        (set `local.EnemyClass` _array_element_2)
        (if (!= _value 0)
          (for _ (range (+ _value 1))
            (bind _returnvalue (`|SpawnActorFromClass` (`local.EnemyClass`) (`KismetMathLibrary.MakeTransform` (`KismetMathLibrary.MakeVector` (+ (`KismetMathLibrary.RandomFloatInRange` -10.0 10.0) _x) 1.0 (+ (`KismetMathLibrary.RandomFloatInRange` -10.0 10.0) _z))) "AdjustIfPossibleButDontSpawnIfColliding" "MultiplyWithRoot" null null))
            (`/Engine/EditorBlueprintResources/StandardMacros.IsValid` _returnvalue
              (:`Is Valid`
                (`KismetArrayLibrary.Array_Add` (`self.EnemiesInRoom`) _returnvalue)))))))))

(fn `UserConstructionScript`)