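; BP_RoomStart is the dungeon generator's start room, which places the main character on BeginPlay.
; After a short delay it finds the first BP_MainCharacter and moves it relative to the StartPoint component.
; X and Z use hardcoded offsets, marked to become half the room size later, while Y is a fixed world value.
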(event `self.ReceiveBeginPlay`
  (bind (_x _y _z) (`KismetMathLibrary.BreakVector3f` (`SceneComponent.K2_GetComponentLocation` (`self.StartPoint`))))
  (`KismetSystemLibrary.Delay` 0.2)
  (bind _outactors (`GameplayStatics.GetAllActorsOfClass` "/Game/Blueprints/Characters/BP_MainCharacter.BP_MainCharacter_C"))
  (`self.K2_SetActorLocation` (`|GetArrayItem` _outactors) (`KismetMathLibrary.MakeVector` (+ _x 320.0) 1.0 (- _z 160.0)) false false))

(fn `UserConstructionScript`)