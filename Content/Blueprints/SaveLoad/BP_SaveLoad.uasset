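; BP_SaveLoad is a data container for saved player stats, modifiers, resources, merchant info and audio settings.
; SaveAllValues copies all gameplay values into member variables in one call, and GetAllValues returns them together.
; SetSFXSettings and GetSFXSettings do the same separately for Master, Sound and Music.
; These functions only store and return values; none of them writes to or reads from a save slot.
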(fn `GetAllValues`
  (returns (MaxHealth :type "Float (double-precision)") (MaxMana :type "Float (double-precision)") (MaxSpeed :type "Float (double-precision)") (Defense :type "Float (double-precision)") (Damage :type "Float (double-precision)") (SpeedMod :type "Float (double-precision)") (DefenseMod :type "Float (double-precision)") (DamageMod :type "Float (double-precision)") (Gold :type Integer) (Chi :type Integer) (Iron :type Integer) (Rice :type Integer) (`Merchant Info` :type "Array of MerchantInfo Structure"))
  (return (`self.MaxHealth`) (`self.MaxMana`) (`self.MaxSpeed`) (`self.Defense`) (`self.Damage`) (`self.SpeedMod`) (`self.DefenseMod`) (`self.DamageMod`) (`self.Gold`) (`self.Chi`) (`self.Iron`) (`self.Rice`) (`self.Merchant Info`)))

(fn `GetSFXSettings`
  (returns (Master :type "Float (double-precision)") (Sound :type "Float (double-precision)") (Music :type "Float (double-precision)"))
  (return (`self.Master`) (`self.Sound`) (`self.Music`)))

(fn `SaveAllValues`
  (params (MaxHealth :type "Float (double-precision)") (MaxMana :type "Float (double-precision)") (MaxSpeed :type "Float (double-precision)") (Defense :type "Float (double-precision)") (Damage :type "Float (double-precision)") (SpeedMod :type "Float (double-precision)") (DefenseMod :type "Float (double-precision)") (DamageMod :type "Float (double-precision)") (Gold :type Integer) (Chi :type Integer) (Iron :type Integer) (Rice :type Integer) (`Merchant Info` :type "Array of MerchantInfo Structure"))
  (`|ExecutionSequence`
    (:`then_0`
      (set `self.MaxHealth` MaxHealth))
    (:`then_1`
      (set `self.MaxMana` MaxMana))
    (:`then_2`
      (set `self.MaxSpeed` MaxSpeed))
    (:`then_3`
      (set `self.Defense` Defense))
    (:`then_4`
      (set `self.Damage` Damage))
    (:`then_5`
      (set `self.SpeedMod` SpeedMod))
    (:`then_6`
      (set `self.DefenseMod` DefenseMod))
    (:`then_7`
      (set `self.DamageMod` DamageMod))
    (:`then_8`
      (set `self.Merchant Info` `Merchant Info`))
    (:`then_9`
      (set `self.Gold` Gold))
    (:`then_10`
      (set `self.Chi` Chi))
    (:`then_11`
      (set `self.Iron` Iron))
    (:`then_12`
      (set `self.Rice` Rice))))

(fn `SetSFXSettings`
  (params (Master :type "Float (double-precision)") (Sound :type "Float (double-precision)") (Music :type "Float (double-precision)"))
  (`|ExecutionSequence`
    (:`then_0`
      (set `self.Master` Master))
    (:`then_1`
      (set `self.Sound` Sound))
    (:`then_2`
      (set `self.Music` Music))))