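; Paper2D mushroom enemy character that patrols along the X axis and can be damaged and killed.
; Tick swaps idle, run and attack flipbooks and moves it, with a forward line trace triggering a pause and reversal through a resettable DoOnce.
; Damage knocks it away from the causer; at zero health it plays hit and dying flipbooks, then destroys itself.
; A looping ChasePlayer event exists but is not called here, and IsEnemyAttacking is only cleared here.
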(event `ChasePlayer`
  (`|AIMoveTo` self (0.0 0.0 0.0) (`GameplayStatics.GetPlayerCharacter` 0) 10.0
    (:`OnSuccess`
      (`KismetSystemLibrary.Delay` 0.2)
      (`self.ChasePlayer`))))

(event `self.ReceiveBeginPlay`
  (set `CharacterMovementComponent.MaxWalkSpeed` (`self.Max Walk Speed`) (`self.CharacterMovement`)))

(event `self.ReceiveTick`
  (params (DeltaSeconds :type "Float (single-precision)"))
  (if (`self.Is Mush Enemy Dead?`)
    _
    (elif (`self.Is Enemy Attacking?`)
      (`PaperFlipbookComponent.SetFlipbook` (`self.Sprite`) (`self.Mushroom_Attack_FB`))
      (`KismetSystemLibrary.Delay` (`PaperFlipbook.GetTotalDuration` (`self.Mushroom_Attack_FB`)))
      (set `self.Is Enemy Attacking?` false)
      (else
        (`self.Animation Update`)
        (`self.Movement Update`)))))

(event `Animation Update`
  ;[1 1 1] Animation Update
  (`PaperFlipbookComponent.SetFlipbook` (`self.Sprite`) (select `bool` (> (`KismetMathLibrary.VSize` (`MovementComponent.Velocity` (`self.CharacterMovement`))) 0.0) :`false` (`self.Mushroom_Idle_FB`) :`true` (`self.Mushroom_Run_FB_0`))))

(event `Movement Update`
  (bind _returnvalue (`self.K2_GetActorLocation`))
  ;[1 1 1] Movement
  (`|ExecutionSequence`
    (:`then_0`
      (if (> (`self.MovementDirection`) 0.0)
        (`self.K2_SetActorRotation` (struct))
        (else
          (`self.K2_SetActorRotation` (struct :`Yaw` 180.0)))))
    (:`then_1`
      (`self.AddMovementInput` (1.0 0.0 0.0) (`self.MovementDirection`))
      (bind (_outhit _returnvalue_2) (`KismetSystemLibrary.LineTraceSingle` _returnvalue (+ (* (`self.GetActorForwardVector`) (300.0 0.0 0.0)) _returnvalue) "TraceTypeQuery1"))
      (if _returnvalue_2
        (`/Engine/EditorBlueprintResources/StandardMacros.DoOnce` false :!label _label
          (:`Completed`
            (set `CharacterMovementComponent.MaxWalkSpeed` 0.0 (`self.CharacterMovement`))
            (`KismetSystemLibrary.Delay` (`self.Duration`))
            (set `CharacterMovementComponent.MaxWalkSpeed` (`self.Max Walk Speed`) (`self.CharacterMovement`))
            (set `self.MovementDirection` (* (`self.MovementDirection`) -1.0))
            (goto _label :!via `Reset`)))))))

(event `self.ReceiveAnyDamage`
  (params (Damage :type "Float (single-precision)") (DamageType :type "DamageType Object Reference") (InstigatedBy :type "Controller Object Reference") (DamageCauser :type "Actor Object Reference"))
  (bind _returnvalue_x (`KismetMathLibrary.BreakVector` (`KismetMathLibrary.Normal` (`KismetMathLibrary.GetDirectionUnitVector` (`self.K2_GetActorLocation` DamageCauser) (`self.K2_GetActorLocation`)))))
  ;[1 1 1] Enemy Damage
  (set `self.Mush_Enemy_Health` (- (`self.Mush_Enemy_Health`) Damage))
  (`self.LaunchCharacter` (`KismetMathLibrary.MakeVector` (* (select `bool` (< _returnvalue_x 0.0) :`false` -1.0 :`true` 1.0) -1500.0)) true true)
  (if (<= (`self.Mush_Enemy_Health`) 0.0)
    (set `self.Is Mush Enemy Dead?` true)
    (`PaperFlipbookComponent.SetFlipbook` (`self.Sprite`) (`self.Mushroom_Hit_FB`))
    (`KismetSystemLibrary.Delay` (`PaperFlipbook.GetTotalDuration` (`self.Mushroom_Hit_FB`)))
    (`PaperFlipbookComponent.SetFlipbook` (`self.Sprite`) (`self.Mushroom_Dying_FB_0`))
    (`ActorComponent.K2_DestroyComponent` (`self.CapsuleComponent`))
    (`KismetSystemLibrary.Delay` 5.0)
    (`self.K2_DestroyActor`)
    (else
      (set `self.Is Mush Enemy Dead?` false))))

(fn `UserConstructionScript`)