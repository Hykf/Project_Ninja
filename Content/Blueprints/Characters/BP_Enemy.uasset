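; Enemy character that damages and knocks back the player and drops money on death.
; A Stats component drives hit and death events, which halt movement, then jump to the GetHit animation or spawn randomly valued BP_Money and disable capsule collision.
; AttackCollision starts disabled; its overlaps call Attack, which deals physical damage to BP_MainCharacter, launches it and flags it as taking damage.
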(event `self.ReceiveBeginPlay`
  (bind _stats (`self.Stats`))
  (set `StatsComponent.MaxHealth` 15.0 _stats)
  (add `StatsComponent.OnDie` _stats (delegate `Death`))
  (add `StatsComponent.OnGetHit` _stats (delegate `Damage`)))

(event `Damage`
  (set `StatsComponent.bIsTakingDamage` true (`self.Stats`))
  (`MovementComponent.StopMovementImmediately` (`self.CharacterMovement`))
  (`CharacterMovementComponent.DisableMovement` (`self.CharacterMovement`))
  (`PaperZDAnimInstance.JumpToNode` (`PaperZDAnimationComponent.AnimInstance` (`self.AnimationComponent`)) "GetHit" "None"))

(event `Death`
  (bind _charactermovement (`self.CharacterMovement`))
  (`|SpawnActorFromClass` "/Game/Blueprints/Collectible/BP_Money.BP_Money_C" (`KismetMathLibrary.MakeTransform` (.location (`self.GetTransform` self)) (.rotation (`self.GetTransform` self)) (/ (.scale (`self.GetTransform` self)) (1.5 1.5 1.5))) "AlwaysSpawn" "MultiplyWithRoot" null (`KismetMathLibrary.RandomIntegerInRange` 10 50) null)
  (set `StatsComponent.bAlive` false (`self.Stats`))
  (`MovementComponent.StopMovementImmediately` _charactermovement)
  (`CharacterMovementComponent.DisableMovement` _charactermovement)
  (`PrimitiveComponent.SetCollisionEnabled` (`self.CapsuleComponent`) "NoCollision"))

(event `self.AttackCollision.OnComponentBeginOverlap`
  (params (OverlappedComponent :type "PrimitiveComponent Object Reference") (OtherActor :type "Actor Object Reference") (OtherComp :type "PrimitiveComponent Object Reference") (OtherBodyIndex :type Integer) (bFromSweep :type Boolean) (SweepResult :type "HitResult Structure (by ref)"))
  (`self.Attack` OtherActor))

(fn `Attack`
  (params (Object :type "Object Object Reference"))
  (set `self.isAttacking` true)
  (bind _asbp_main_character (cast `/Game/Blueprints/Characters/BP_MainCharacter` Object))
  (`/Game/Blueprints/Characters/BP_MainCharacter.Deal Damage` _asbp_main_character _asbp_main_character "Physical" (`StatsComponent.Damage` (`self.Stats`)))
  (`self.LaunchCharacter` _asbp_main_character (+ (* (`self.GetActorForwardVector` self) (50.0 0.0 100.0)) (0.0 0.0 100.0)) false false)
  (set `StatsComponent.bIsTakingDamage` true (`CharacterBase.Stats` _asbp_main_character)))

(fn `UserConstructionScript`
  (`PrimitiveComponent.SetCollisionEnabled` (`self.AttackCollision`) "NoCollision"))