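; BP_BOX is a breakable wooden box that rewards the player with rice when destroyed.
; On begin play, its sprite stops and becomes visible after a short random delay; construction assigns the box-specific Niagara hit effect.
; Stats.OnDie disables collision, adds Value to the main character's TreasureComponent, spawns floating amount text, destroys the box and plays a breaking sound.
; A separate CustomEvent, uncalled here, spawns a scaled-down BP_Rice with random value.
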(event `self.ReceiveBeginPlay`
  (bind _sprite (`self.Sprite`))
  (`KismetSystemLibrary.Delay` (`KismetMathLibrary.RandomFloatInRange` 0.1 1.0))
  (`PaperFlipbookComponent.Stop` _sprite)
  (`SceneComponent.SetVisibility` _sprite true false))

(event `self.Stats.OnDie`
  (bind _value (`self.Value`))
  (`PrimitiveComponent.SetCollisionEnabled` (`self.BoxCollision`) "NoCollision")
  (bind _outactors (`GameplayStatics.GetAllActorsOfClass` "/Game/Blueprints/Characters/BP_MainCharacter.BP_MainCharacter_C"))
  (`TreasureComponent.AddRice` (`MainCharacter.TreasureComponent` (`|GetArrayItem` _outactors)) _value)
  (`|SpawnActorFromClass` "/Game/Blueprints/Collectible/BP_FloatingText.BP_FloatingText_C" (`self.GetTransform` self) "AlwaysSpawn" "MultiplyWithRoot" null (`KismetTextLibrary.Conv_IntToText` _value) (struct :`R` 0.302083 :`G` 0.207981 :`B` 0.133214 :`A` 1.0) false null)
  (`self.K2_DestroyActor`)
  (`GameplayStatics.PlaySound2D` "/Game/StarterContent/Audio/breakingWood_Cue.breakingWood_Cue" 1.0 1.0 0.0 null null))

(event `CustomEvent`
  (`|SpawnActorFromClass` "/Game/Blueprints/Collectible/BP_Rice.BP_Rice_C" (`KismetMathLibrary.MakeTransform` (.location (`self.GetTransform` self)) (.rotation (`self.GetTransform` self)) (/ (.scale (`self.GetTransform` self)) (1.5 1.5 1.5))) "AlwaysSpawn" "MultiplyWithRoot" null (`KismetMathLibrary.RandomIntegerInRange` 10 50) null))

(fn `UserConstructionScript`
  (`parent.UserConstructionScript`)
  (set `self.GetHitVFEffect` "/Game/PixelArt/Character/Main/NS_GetHit_Box.NS_GetHit_Box"))