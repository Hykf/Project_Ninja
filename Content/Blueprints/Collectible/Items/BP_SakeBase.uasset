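; Base Blueprint for sake collectible items, which heal the character that uses them.
; On BeginPlay it looks up the Tavern merchant in BP_GameInstance and multiplies SakeValue by that merchant's current level plus one.
; UseItem passes the scaled value to the character's Stats as healing, so the Tavern's level at spawn sets the heal strength.
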(event `self.ReceiveBeginPlay`
  (bind _asbp_game_instance (cast `/Game/Blueprints/Characters/BP_GameInstance` (`GameplayStatics.GetGameInstance`)))
  (bind _array_element (`/Game/Blueprints/Characters/BP_GameInstance.FindMerchantByName` _asbp_game_instance "Tavern"))
  (set `self.SakeValue` (* (`self.SakeValue`) (+ (`.CurrentLevel` (break `MerchantInfo` _array_element)) 1))))

(event `self.UseItem`
  (params (Character :type "CharacterBase Object Reference"))
  (`StatsComponent.ReceiveHealing` (`CharacterBase.Stats` Character) (`self.SakeValue`)))

(fn `UserConstructionScript`)