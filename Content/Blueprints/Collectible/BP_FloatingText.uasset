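; BP_FloatingText is a short-lived actor that shows floating text, such as damage or other feedback, through a DamageIndicator widget component.
; On BeginPlay it passes its Text, Color and IsDamage variables to the component's WBP_DamageIndicator widget via SetDamageText.
; It then destroys itself after a fixed five-second delay.
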(event `self.ReceiveBeginPlay`
  (`self.DisplayDamageIndicator`)
  (`KismetSystemLibrary.Delay` 5.0)
  (`self.K2_DestroyActor`))

(fn `DisplayDamageIndicator`
  (bind _aswbp_damage_indicator (cast `/Game/Blueprints/Widgets/WBP_DamageIndicator` (`WidgetComponent.GetWidget` (`self.DamageIndicator`))))
  (`/Game/Blueprints/Widgets/WBP_DamageIndicator.SetDamageText` _aswbp_damage_indicator (`self.Text`) (`self.Color`) (`self.isDamage`)))

(fn `UserConstructionScript`)